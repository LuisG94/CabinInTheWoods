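; First-person player pawn Blueprint that handles basic movement and mouse-look style input.
; Four axis events feed movement and look: forward/back and strafe call AddMovementInput, while the look axes add controller yaw and pitch.
; Movement directions come from the full control rotation, so the forward vector includes camera pitch rather than being flattened to yaw.
; The construction script is empty.
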(event Input|AxisEvents|InputAxisForwards_Backwards
  (params (AxisValue :type Float%20%28single-precision%29))
  ;[1 1 1] Forward_Backword
  (Pawn|Input|AddMovementInput (Math|Vector|GetForwardVector (Pawn|GetControlRotation :!class /Script/Engine.Pawn)) AxisValue false))

(event Input|AxisEvents|InputAxisLeft_Right
  (params (AxisValue :type Float%20%28single-precision%29))
  ;[1 1 1] Left_Right
  (Pawn|Input|AddMovementInput (Math|Vector|GetRightVector (Pawn|GetControlRotation :!class /Script/Engine.Pawn)) AxisValue false))

(event Input|AxisEvents|InputAxisLook_Left_Right
  (params (AxisValue :type Float%20%28single-precision%29))
  ;[1 1 1] Comment
  (Pawn|Input|AddControllerYawInput AxisValue))

(event Input|AxisEvents|InputAxisLook_Up_Down
  (params (AxisValue :type Float%20%28single-precision%29))
  ;[1 1 1] Comment
  (Pawn|Input|AddControllerPitchInput AxisValue))

(fn ConstructionScript)