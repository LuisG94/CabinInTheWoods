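; Base door Blueprint that swings its Scene component open and closed by a normalized open value.
; SetOpenValue clamps the requested value and plays or reverses the UpdateOpenValue timeline depending on whether it exceeds the current value.
; Each timeline update sets relative yaw to the current value scaled by MaxOpenDeg, stopping near the target to allow partial opening.
; The construction script calls SetDuration, which sets timeline play rate to the reciprocal of Duration.
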(event Custom|SetOpenValue
  (params (newOpenValue :type Float%20%28single-precision%29))
  (Utilities|FlowControl|Sequence
    (:then_0
      (bind _newvalue (Timeline|UpdateOpenValue Stop)
        (:Update
          (bind _output_get (Variables|DoorSetup|SetcurrOpenValue _newvalue))
          (Transformation|SetRelativeRotation (Variables|Default|GetScene) (Math|Rotator|MakeRotator 0.0 0.0 (* _output_get (Variables|DoorSetup|GetmaxOpenDeg))) false false)
          (if (Math|Float|NearlyEqual(Float) (Variables|DoorSetup|GetnewOpenValue) (Variables|DoorSetup|GetcurrOpenValue) 0.01)
            (Timeline|UpdateOpenValue Stop)))))
    (:then_1
      (bind _output_get_2 (Variables|DoorSetup|SetnewOpenValue (Math|Float|Clamp(Float) newOpenValue)))
      (if (> _output_get_2 (Variables|DoorSetup|GetcurrOpenValue))
        (Timeline|UpdateOpenValue Play)
        (else
          (Timeline|UpdateOpenValue Reverse))))))

(fn ConstructionScript
  (CallFunction|SetDuration (Variables|DoorSetup|GetDuration)))

(fn SetDuration
  (params (newDuration :type Float%20%28single-precision%29))
  (bind _output_get (Variables|DoorSetup|SetDuration newDuration))
  (Components|Timeline|SetPlayRate (Variables|Default|GetUpdateOpenValue) (/ (Math|Float|MakeLiteralFloat 1.0) _output_get)))